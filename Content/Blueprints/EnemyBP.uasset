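; Enemy fighter Blueprint with basic AI that plays a selectable US president, spawns a health bar and opens the "Won" level when its health runs out.
; Game mode and GameInstance settings pick the mesh and AnimBP.
; On seeing the player it loops AIMoveTo into random kicks or per-character punches, applying range-checked damage halfway through most montages.
; Kennedy has separate combo logic with a weakened wandering phase.
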(event `self.ReceiveTick`
  (params (DeltaSeconds :type "Float (single-precision)"))
  ;[1 1 1] Basic Dummy AI
  (if (<= (`self.CurrentHealth`) 0.0)
    (set `self.CurrentHealth` 0.0)
    (`GameplayStatics.OpenLevel` "Won")
    (set `self.isDead` true)
    (if (not (`self.isDead`))
      (if (`self.freshStart`)
        (set `self.freshStart` false)
        (else
          (`KismetSystemLibrary.Delay` 1.0)))
      (`self.ChasePlayer` (`GameplayStatics.GetPlayerCharacter` 0)))))

(event `ChasePlayer`
  (params (PlayerToChase :type "Pawn Object Reference"))
  ;[1 1 1] Basic Dummy AI
  (`|AIMoveTo` self (0.0 0.0 0.0) PlayerToChase 120.0
    (:`OnSuccess`
      (if (not (`self.isAttacking`))
        (`self.UpdateRange`)
        (if (== (`KismetMathLibrary.RandomIntegerInRange` 0 6) 0)
          (`self.KickAttack`)
          (else
            (`self.PunchAttack`
              (:`then`
                _)
              (:`then 2`
                _)
              (:`then 3`
                _)
              (:`then 4`
                _)
              (:`then 5`
                _)
              (:`then 6`
                _))))
        (set `self.isAttacking` false)
        (`self.ChasePlayer` (`GameplayStatics.GetPlayerCharacter` 0))))))

(event `self.ReceiveAnyDamage`
  (params (Damage :type "Float (single-precision)") (DamageType :type "DamageType Object Reference") (InstigatedBy :type "Controller Object Reference") (DamageCauser :type "Actor Object Reference"))
  ;[1 1 1] Calculates Damage
  (set `self.CurrentHealth` (- (`self.CurrentHealth`) Damage)))

(event `self.ReceiveBeginPlay`
  ;[1 1 1] Character Select / Health Bar
  (`self.GameModeSelected`)
  (bind _returnvalue (`|CreateWidget` "/Game/UI/EnemyHealthBar.EnemyHealthBar_C"))
  (`UserWidget.AddToViewport` _returnvalue 0)
  (bind _outactors (`GameplayStatics.GetAllActorsOfClass` "/Game/Blueprints/0-Player/ChPlayer.ChPlayer_C"))
  (for _array_element _outactors
    (set `self.PlayerCharacter` _array_element)))

(event `self.PawnSensing.OnSeePawn`
  (params (Pawn :type "Pawn Object Reference"))
  ;[1 1 1] Chase on sight, might need to change later
  (bind _asch_player (cast `/Game/Blueprints/0-Player/ChPlayer` Pawn))
  (`self.ChasePlayer` _asch_player))

(fn `BushPunching`
  (returns (Delay :type "Float (double-precision)"))
  (if (not (`self.isAttacking`))
    (set `self.isAttacking` true)
    (switch `int` (`KismetMathLibrary.RandomIntegerInRange` 0 1)
      (:`0`
        (bind _returnvalue (`self.PlayAnimMontage` "/Game/Characters/Bush/BushZombie_Punching__1__Montage.BushZombie_Punching__1__Montage"))
        (set `self.Delay Time` _returnvalue)
        (set `self.Damage` 10.0))
      (:`1`
        (bind _returnvalue_2 (`self.PlayAnimMontage` "/Game/Characters/Bush/BushZombie_Punching_Montage.BushZombie_Punching_Montage"))
        (set `self.Delay Time` _returnvalue_2)
        (set `self.Damage` 11.0)))
    (`self.UpdateRange`)
    (return (/ (`self.Delay Time`) 2.0))))

(fn `DamagePlayer`
  (if (`self.isInRange`)
    (if (`self.isAttacking`)
      (`GameplayStatics.ApplyDamage` (`self.PlayerCharacter`) (`self.Damage`)))))

(fn `GameModeSelected`
  (bind _character (`self.Character`))
  (bind _returnvalue (`GameplayStatics.GetCurrentLevelName` true))
  (if (`KismetStringLibrary.EqualEqual_StrStr` _returnvalue "PvESelect")
    (bind _asmy_game_instance (cast `/Game/Blueprints/MyGameInstance` (`GameplayStatics.GetGameInstance`)))
    (`self.SetCharacter` (`/Game/Blueprints/MyGameInstance.ECharacter` _asmy_game_instance))
    (else
      (bind _asmy_game_instance_2 (cast `/Game/Blueprints/MyGameInstance` (`GameplayStatics.GetGameInstance`)))
      (if (`/Game/Blueprints/MyGameInstance.CampaignMode` _asmy_game_instance_2)
        (`self.SetCharacter` _character :!label _label)
        (else
          (bind _echaracter (`/Game/Blueprints/MyGameInstance.ECharacter` _asmy_game_instance_2))
          (if (== _echaracter "None")
            (goto _label)
            (else
              (`self.SetCharacter` _echaracter)
              (`self.SetCharacter` _character))))))))

(fn `KennedyPunching`)

(fn `LincolnPunching`
  (returns (Delay :type "Float (double-precision)"))
  (if (not (`self.isAttacking`))
    (set `self.isAttacking` true)
    (switch `int` (`KismetMathLibrary.RandomIntegerInRange` 0 1)
      (:`0`
        (bind _returnvalue (`self.PlayAnimMontage` "/Game/Characters/Lincoln/LincolnAnimation/LincolnCross_Punch__1__Montage.LincolnCross_Punch__1__Montage"))
        (set `self.Delay Time` _returnvalue)
        (set `self.Damage` 14.0))
      (:`1`
        (bind _returnvalue_2 (`self.PlayAnimMontage` "/Game/Characters/Lincoln/LincolnAnimation/LincolnPunching__2__Montage.LincolnPunching__2__Montage"))
        (set `self.Delay Time` _returnvalue_2)
        (set `self.Damage` 8.0)))
    (`self.UpdateRange`)
    (return (/ (`self.Delay Time`) 2.0))))

(fn `ObamaPunching`
  (returns (Delay :type "Float (double-precision)"))
  (if (not (`self.isAttacking`))
    (set `self.isAttacking` false)
    (switch `int` (`KismetMathLibrary.RandomIntegerInRange` 0 1)
      (:`0`
        (bind _returnvalue (`self.PlayAnimMontage` "/Game/Characters/Obama/NewObamaAnimations/ObamaHook_Punch_Montage.ObamaHook_Punch_Montage"))
        (set `self.Delay Time` _returnvalue)
        (set `self.Damage` 12.0))
      (:`1`
        (bind _returnvalue_2 (`self.PlayAnimMontage` "/Game/Characters/Obama/NewObamaAnimations/ObamaPunching_Montage.ObamaPunching_Montage"))
        (set `self.Delay Time` _returnvalue_2)
        (set `self.Damage` 10.0)))
    (`self.UpdateRange`)
    (return (/ (`self.Delay Time`) 2.0))))

(fn `SetCharacter`
  (params (CharacterName :type Name))
  (if (== CharacterName "Trump")
    (`SkinnedMeshComponent.SetSkinnedAssetAndUpdate` (`self.Mesh`) "/Game/Characters/Trump1/newTrump/Donald_Trump_animation.Donald_Trump_animation" true)
    (`SkeletalMeshComponent.K2_SetAnimInstanceClass` (`self.Mesh`) "/Game/Characters/Trump1/TrumpAnimBP.TrumpAnimBP_C")
    (elif (== CharacterName "Obama")
      (`SkinnedMeshComponent.SetSkinnedAssetAndUpdate` (`self.Mesh`) "/Game/Characters/Obama/Obama_animation_1_.Obama_animation_1_" true)
      (`SkeletalMeshComponent.K2_SetAnimInstanceClass` (`self.Mesh`) "/Game/Characters/Obama/NewObamaAnimations/NewObamaAnimBP.NewObamaAnimBP_C")
      (elif (== CharacterName "Bush")
        (`SkinnedMeshComponent.SetSkinnedAssetAndUpdate` (`self.Mesh`) "/Game/Characters/Bush/Bush/George_W_Bush__animated.George_W_Bush__animated" true)
        (`SkeletalMeshComponent.K2_SetAnimInstanceClass` (`self.Mesh`) "/Game/Characters/Bush/BushAnimBP.BushAnimBP_C")
        (elif (== CharacterName "Lincoln")
          (`SkinnedMeshComponent.SetSkinnedAssetAndUpdate` (`self.Mesh`) "/Game/Characters/Lincoln/Lincoln/Abraham_Lincoln_mecanim_rig.Abraham_Lincoln_mecanim_rig" true)
          (`SkeletalMeshComponent.K2_SetAnimInstanceClass` (`self.Mesh`) "/Game/Characters/Lincoln/LincolnAnimBP.LincolnAnimBP_C")
          (elif (== CharacterName "Kennedy")
            (`SkinnedMeshComponent.SetSkinnedAssetAndUpdate` (`self.Mesh`) "/Game/Characters/JFK/JFK/JFK_animation1.JFK_animation1" true)
            (`SkeletalMeshComponent.K2_SetAnimInstanceClass` (`self.Mesh`) "/Game/Characters/JFK/JFKAnimBP.JFKAnimBP_C")))))))

(fn `TrumpPunching`
  (returns (Delay :type "Float (double-precision)"))
  (if (not (`self.isAttacking`))
    (set `self.isAttacking` true)
    (switch `int` (`KismetMathLibrary.RandomIntegerInRange` 0 1)
      (:`0`
        (bind _returnvalue (`self.PlayAnimMontage` "/Game/Characters/Trump1/TrumpAnimations/Right_Hook_Montage.Right_Hook_Montage"))
        (set `self.Delay Time` _returnvalue)
        (set `self.Damage` 12.0))
      (:`1`
        (bind _returnvalue_2 (`self.PlayAnimMontage` "/Game/Characters/Trump1/TrumpAnimations/Uppercut_Montage.Uppercut_Montage"))
        (set `self.Delay Time` _returnvalue_2)
        (set `self.Damage` 15.0)))
    (`self.UpdateRange`)
    (return (/ (`self.Delay Time`) 2.0))))

(fn `UpdateRange`
  (bind _output_get (set `self.isInRange` (<= (`self.GetDistanceTo` (`self.PlayerCharacter`)) (`self.Range`))))
  (if _output_get
    _))

(fn `UserConstructionScript`)